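; GA_TargetedBase is a base gameplay ability for player-confirmed, ground or area targeting with a 200-unit radius.
; On activation it waits on the GAR_Area_200 targeting actor, commits, then sphere-overlaps pawns at the confirmed point, excluding the caster unless CanTargetSelf is set.
; Each hit pawn goes to the ApplyToTarget event, which here only prints a debug message.
; Confirming or cancelling both end the ability.
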(event Custom|ApplyToTarget
  (params (TargetActor :type Actor%20Object%20Reference))
  ;[0.15 0.15 0.15 0.5] Comment
  (Development|PrintString (Utilities|String|Append (Utilities|GetDisplayName TargetActor) "is hit！") true true "(R=0.000000,G=0.660000,B=1.000000,A=1.000000)" 1e+01))

(event Ability|EventActivateAbility
  (bind _data (|WaitTargetData :ConfirmationType "UserConfirmed" :Class "/Game/Ability/GAR_Area_200.GAR_Area_200_C" :TraceProfile "(Name=\"BlockAllDynamic\")" :StartLocation (Utilities|Struct|MakeGameplayAbilityTargetingLocationInfo (Ability|GetAvatarActorfromActorInfo) 0 self "0.000000,0.000000,0.000000|0.000000,0.000000,-0.000000|1.000000,1.000000,1.000000" "None" "ActorTransform") :ReticleClass 0)
    (:ValidData
      (Ability|CommitAbility)
      (bind _outactors (Collision|SphereOverlapActors (Class|AbilitySystemBlueprintLibrary|GetTargetDataEndPoint _data) 2e+02 (Utilities|Array|MakeArray "ObjectTypeQuery3") 0 (select (Variables|Default|GetCanTargetSelf) 0 (Utilities|Array|MakeArray (Ability|GetAvatarActorfromActorInfo)))))
      (for _array_element _outactors
        (CallFunction|ApplytoTarget _array_element)))
    (:Cancelled
      (Development|PrintString "Cancelled" true true "(R=0.000000,G=0.660000,B=1.000000,A=1.000000)" 1e+01)))
  (Ability|EndAbility))